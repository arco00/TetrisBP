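; Movable falling block for a Tetris-style grid game, providing move, slide, placement and line-clear functions for other code to call.
; Moves step 100 units, with X as height and Y as column, validated against board bounds and the dead blocks listed in BP_Saver.
; Landed blocks spawn as tinted dead actors registered in the saver.
; Full rows leave that list, and their heights are queued for lowering.
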(event EventBeginPlay
  (bind _returnvalue (Actor|GetActorOfClass "/Game/BP/BP_Saver.BP_Saver_C"))
  (Variables|Default|Setsaver _returnvalue))

(event Collision|EventActorBeginOverlap
  (params (OtherActor :type Actor%20Object%20Reference)))

(event EventTick
  (params (DeltaSeconds :type Float%20%28single-precision%29)))

(fn ConstructionScript)

(fn DownCheck
  (bind _in (CallFunction|CheckMove (Math|Vector|MakeVector -1e+02 0.0 0.0)))
  (return _in))

(fn CheckOutOfBound
  (params (direction :type Vector))
  (return (Math|Boolean|ANDBoolean (>= (.x direction) 0.0) (>= (.y direction) 0.0) (<= (.y direction) (* (Variables|Default|Getlargeur) 1e+02)))))

(fn CheckDeadBlock
  (params (direction :type Vector))
  (Variables|Default|SetemptyLoc true)
  (for _array_element (Variables|/Game/BP/BP_Saver.BP_Saver_C|GetdeadList (Variables|Default|Getsaver))
    (if (Utilities|Operators|EqualEqual direction (Transformation|GetActorLocation _array_element) 1e+01)
      (Variables|Default|SetemptyLoc false)))
  (return (Variables|Default|GetemptyLoc)))

(fn MoveBlock
  (params (movement :type Vector))
  (Transformation|SetActorLocation (+ movement (Transformation|GetActorLocation)) false false))

(fn SpawnDeadBlock
  (params (actor :type Actor%20Object%20Reference))
  (bind _returnvalue (Game|SpawnActorfromClass (Variables|Default|GetclassDead) (Transformation|GetActorTransform actor) "Undefined" "MultiplyWithRoot" 0 0))
  (bind _returnvalue_2 (Rendering|Material|CreateDynamicMaterialInstance (Variables|/Game/BP/BP_DeadBlock.BP_DeadBlock_C|GetPlane _returnvalue) 0 0 "None" :!class /Script/Engine.PrimitiveComponent))
  (Rendering|Material|SetVectorParameterValue _returnvalue_2 (Variables|Default|GetcolorBase) (Variables|/Game/BP/BP_Saver.BP_Saver_C|GetactualColor (Variables|Default|Getsaver)) :!class /Script/Engine.MaterialInstanceDynamic)
  (Default|AddtoDeadList (Variables|Default|Getsaver) _returnvalue))

(fn SlideCheck
  (params (input :type Float%20%28double-precision%29))
  (bind _in (CallFunction|CheckMove (Math|Vector|MakeVector 0.0 (* input 1e+02) 0.0)))
  (return _in))

(fn PlaceBlock
  (params (changemenSpawn :type Vector))
  (Transformation|SetActorLocation (+ changemenSpawn (Variables|Default|GetspawnPoint)) false false))

(fn TestLineFull
  (params (newDeadBlock :type Actor%20Object%20Reference))
  (bind _returnvalue (Transformation|GetActorLocation newDeadBlock))
  (bind _templist (LocalVariables|GettempList))
  (for _array_element (Variables|/Game/BP/BP_Saver.BP_Saver_C|GetdeadList (Variables|Default|Getsaver))
    (if (== (.x _returnvalue) (.x (Transformation|GetActorLocation _array_element)))
      (Utilities|Array|AddUnique _templist _array_element)
      (if (== (+ (Utilities|Array|Length _templist) -1) (Variables|Default|Getlargeur))
        (for _array_element_2 (LocalVariables|GettempList)
          (bind _asbp_dead_block (Utilities|Casting|CastToBP_DeadBlock _array_element_2))
          (Default|RemovefromDeadList (Variables|Default|Getsaver) _asbp_dead_block))
        (Utilities|Array|AddUnique (Variables|/Game/BP/BP_Saver.BP_Saver_C|GetlistLineToLower (Variables|Default|Getsaver)) (.x _returnvalue))))))

(fn CheckMove
  (params (direction :type Vector))
  (bind _returnvalue (Transformation|GetActorLocation))
  (bind _returnvalue_2 (+ direction _returnvalue))
  (bind _in (CallFunction|CheckOutOfBound _returnvalue_2))
  (bind _empty (CallFunction|CheckDeadBlock _returnvalue_2))
  (return (and _empty _in)))